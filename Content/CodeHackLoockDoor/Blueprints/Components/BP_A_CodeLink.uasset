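; BP_A_CodeLink is a visual link piece for the code-hack door lock that shows its status through a holographic cube.
; SetState switches on a state value to hide the cube or show it with a default, red or green emissive hologram material, then stores that state.
; It has no active logic of its own, so state changes come only from calls to SetState.
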(event Custom|SetState
  (params (State :type Integer))
  (bind _cube (Variables|Default|GetCube))
  (bind _cube_2 (Variables|Default|GetCube))
  (switch int State
    (:0
      (Rendering|SetVisibility _cube false false))
    (:1
      (Rendering|SetVisibility _cube true false)
      (Rendering|Material|SetMaterial _cube_2 0 "/Game/CodeHackLoockDoor/Materials/M_DefaultMaterialGalogramEmissive.M_DefaultMaterialGalogramEmissive"))
    (:2
      (Rendering|SetVisibility _cube true false)
      (Rendering|Material|SetMaterial _cube_2 0 "/Game/CodeHackLoockDoor/Materials/MI_DefaultMaterialGalogramEmissive_InstRed.MI_DefaultMaterialGalogramEmissive_InstRed"))
    (:3
      (Rendering|SetVisibility _cube true false)
      (Rendering|Material|SetMaterial _cube_2 0 "/Game/CodeHackLoockDoor/Materials/MI_DefaultMaterialGalogramEmissive_InstGreen.MI_DefaultMaterialGalogramEmissive_InstGreen")))
  (Variables|Default|SetState State))

(event EventBeginPlay)

(event Collision|EventActorBeginOverlap
  (params (OtherActor :type Actor%20Object%20Reference)))

(event EventTick
  (params (DeltaSeconds :type Float%20%28single-precision%29)))

(fn ConstructionScript)