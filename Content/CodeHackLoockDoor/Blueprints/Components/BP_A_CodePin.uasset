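; BP_A_CodePin is a single pin actor for the code-hack lock, showing an on or off state through its mesh material.
; SetState stores the boolean and swaps MeshPin between two emissive materials, starting off at BeginPlay, and GetState returns the value.
; Pawn interactions through BPI_InteractionPawn are forwarded to the owning BP_CodeHacked, so the pin holds no interaction logic of its own.
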(event Custom|SetState
  (params (On :type Boolean))
  (bind _meshpin (Variables|Default|GetMeshPin))
  (bind _output_get (Variables|Default|SetState On))
  (if _output_get
    (Rendering|Material|SetMaterial _meshpin 0 "/Game/CodeHackLoockDoor/Materials/MI_DefaultMaterialEmissive_Inst1.MI_DefaultMaterialEmissive_Inst1")
    (else
      (Rendering|Material|SetMaterial _meshpin 0 "/Game/CodeHackLoockDoor/Materials/M_DefaultMaterialEmissive.M_DefaultMaterialEmissive"))))

(event EventBeginPlay
  (CallFunction|SetState false))

(event Collision|EventActorBeginOverlap
  (params (OtherActor :type Actor%20Object%20Reference)))

(event EventTick
  (params (DeltaSeconds :type Float%20%28single-precision%29)))

(fn ConstructionScript)

(fn GetState
  (return (Variables|Default|GetState)))

(fn BPIInteractionPawn
  (params (Pawn :type Pawn%20Object%20Reference))
  (bind _asbp_code_hacked (Utilities|Casting|CastToBP_CodeHacked (Components|GetOwner)))
  (bind _isinteraction (CallFunction|BPIInteractionPawn _asbp_code_hacked Pawn))
  (return _isinteraction))